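; Visual novel script manager that shows a loading screen, builds the HUD and steps through a data-driven story on left click.
; Each script row sets music, background and an event type: dialog, focused image pop-up, fade-in or background change.
; Dialog and focused events read a separately counted dialog table for name, line, expression and SFX.
; The Proceed flag gates clicks, while MsgEnd restores the prompt, with extra checks for focused events.
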(event `self.ReceiveBeginPlay`
  (bind _returnvalue (`|CreateWidget` "/Game/UI/WG_Loading.WG_Loading_C" (`GameplayStatics.GetPlayerController` 0)))
  (bind _output_get (set `self.LoadingScreen` _returnvalue))
  (`UserWidget.AddToViewport` _output_get 0)
  (`KismetSystemLibrary.Delay` 2.0)
  (bind _returnvalue_2 (`|CreateWidget` "/Game/UI/WG_Hud.WG_Hud_C" (`GameplayStatics.GetPlayerController` 0) self))
  (set `self.HudRef` _returnvalue_2)
  (`Widget.RemoveFromParent` (`self.LoadingScreen`))
  (`UserWidget.AddToViewport` (`self.HudRef`) 0)
  (`self.GetScriptRow` "1")
  (`|ExecutionSequence`
    (:`then_0`
      (`self.Play Music`))
    (:`then_1`
      (`KismetSystemLibrary.Delay` 1.0)
      (`/Game/UI/WG_Dialog.Show Dialog` (`/Game/UI/WG_Hud.WG_Dialog` (`self.HudRef`))))))

(event `Key|LeftMouseButton`
  (params (Key :type "Key Structure"))
  ;[1 1 1] 输入
  (:`Pressed`
    (if (`self.Proceed`)
      (`self.Action`))))

(event `Action`
  (bind _wg_dialog (`/Game/UI/WG_Hud.WG_Dialog` (`self.HudRef`)))
  ;[1 1 1] 执行动作
  (set `self.Proceed` false)
  (`/Game/UI/WG_Dialog.ClearText` _wg_dialog)
  (`/Game/UI/WG_Dialog.ShowProceed` _wg_dialog "Hidden")
  (`self.NextScriptRow`)
  (`self.GetScriptRow` (`KismetStringLibrary.Conv_StringToName` (`KismetStringLibrary.Conv_IntToString` (`self.ScriptCounter`))))
  (`|ExecutionSequence`
    (:`then_0`
      (switch `/Game/BluePrint/Enums/E_Scripts` (`self.Epecial Event`)
        (:`NewEnumerator1`
          (`self.FocusedEvent`))
        (:`NewEnumerator2`
          (`self.PlayMsg`))
        (:`NewEnumerator5`
          (`self.FadeInEvent`))
        (:`NewEnumerator6`
          (`self.ChangeBackground`))))
    (:`then_1`
      ;[1 1 1] 如果音乐正在播放则切换
      (if (not (== (`self.ScriptCounter`) 1))
        (`self.Play Music`)))))

(event `PlayMsg`
  ;[1 1 1] 对话开始Dialog
  (`self.NextDialogRow`)
  (`self.GetDialogRow`)
  (set `self.Typing` true)
  (`|ExecutionSequence`
    (:`then_0`
      (`/Engine/EditorBlueprintResources/StandardMacros.IsValid` (`self.SFX`)
        (:`Is Valid`
          (`GameplayStatics.PlaySound2D` (`self.SFX`) 1.0 1.0 0.0 null null))))
    (:`then_1`
      (`self.SetCharacterExpression`)
      (`/Game/UI/WG_Dialog.StartMsg` (`/Game/UI/WG_Hud.WG_Dialog` (`self.HudRef`)) (`self.Name`) (`self.Line`)))))

(event `MsgEnd`
  ;[1 1 1] 对话结束
  (set `self.Typing` false)
  (switch `/Game/BluePrint/Enums/E_Scripts` (`self.Epecial Event`)
    (:`NewEnumerator1`
      (`self.FocusedEventProceed`))
    (:`NewEnumerator2`
      (`/Game/UI/WG_Dialog.ShowProceed` (`/Game/UI/WG_Hud.WG_Dialog` (`self.HudRef`)) "Visible" :!label _label)
      (`self.EnableInputAfterFirstRun`))
    (:`NewEnumerator5`
      (goto _label))
    (:`NewEnumerator6`
      (goto _label))))

(event `FadeInEvent`
  (bind _hudref (`self.HudRef`))
  (bind _background (`self.Background`))
  ;[1 1 1] 渐入渐出事件FadeIn
  (`|ExecutionSequence`
    (:`then_0`
      (`/Engine/EditorBlueprintResources/StandardMacros.IsValid` _background
        (:`Is Valid`
          (`Image.SetBrushFromTexture` (`/Game/UI/WG_Hud.Background` (`self.HudRef`)) _background false))))
    (:`then_1`
      (`/Game/UI/WG_Dialog.ClearText` (`/Game/UI/WG_Hud.WG_Dialog` _hudref))
      (`/Game/UI/WG_Fade.FadeInAnimationPlay` (`/Game/UI/WG_Hud.WG_Fade` _hudref)))))

(event `FocusedEvent`
  (bind _hudref (`self.HudRef`))
  ;[1 1 1] 注视事件Focused
  (`self.PlayMsg`)
  (set `self.FocusedActive` true)
  (set `self.Focusing？` true)
  (`/Game/UI/WG_FocusedEvent.PlayPopAnimation` (`/Game/UI/WG_Hud.WG_FocusedEvent` _hudref) "Forward" (`|GetArrayItem` (`self.FocusedEventImage`) (`self.FocusedCounter`)))
  (`/Engine/EditorBlueprintResources/StandardMacros.IncrementInt` (`self.FocusedCounter`)
    (:`  `
      (`Widget.SetVisibility` (`/Game/UI/WG_Hud.BackgroundBlur` _hudref) "Visible"))))

(event `HideFocusedEvent`
  (bind _hudref (`self.HudRef`))
  ;[1 1 1] 隐藏注视事件
  (if (`self.FocusedActive`)
    (`/Game/UI/WG_FocusedEvent.PlayPopAnimation` (`/Game/UI/WG_Hud.WG_FocusedEvent` _hudref) "Reverse" null)
    (`Widget.SetVisibility` (`/Game/UI/WG_Hud.BackgroundBlur` _hudref) "Hidden")
    (set `self.FocusedActive` false)))

(event `ChangeBackground`
  (bind _background (`self.Background`))
  (bind _hudref (`self.HudRef`))
  ;[1 1 1] 切换背景ChangeBackground
  (`self.HideFocusedEvent`)
  (`/Game/UI/WG_Dialog.Hide Dialog` (`/Game/UI/WG_Hud.WG_Dialog` _hudref))
  (`Widget.SetVisibility` (`/Game/UI/WG_Character01.CharacterImage` (`/Game/UI/WG_Hud.WG_Character01` _hudref)) "Hidden")
  (`/Game/UI/WG_Fade.FadeOutAnimationPlay` (`/Game/UI/WG_Hud.WG_Fade` _hudref))
  (`KismetSystemLibrary.Delay` 0.5)
  (`/Engine/EditorBlueprintResources/StandardMacros.IsValid` _background
    (:`Is Valid`
      (`Image.SetBrushFromTexture` (`/Game/UI/WG_Hud.Background` (`self.HudRef`)) _background false))))

(event `YesNo`)

(fn `EnableInputAfterFirstRun`
  (bind _returnvalue (`GameplayStatics.GetPlayerController` 0))
  (if (== (`self.ScriptCounter`) 1)
    (`self.EnableInput` _returnvalue)
    (set `PlayerController.bShowMouseCursor` true _returnvalue)))

(fn `FocusedEventProceed`
  (if (`self.Typing`)
    _
    (elif (not (`self.Focusing？`))
      (`/Game/UI/WG_Dialog.ShowProceed` (`/Game/UI/WG_Hud.WG_Dialog` (`self.HudRef`)) "Visible"))))

(fn `GetDialogRow`
  (bind _returnvalue (`|GetDataTableRow` (`self.DT_Dialog`) (`KismetStringLibrary.Conv_StringToName` (`KismetStringLibrary.Conv_IntToString` (`self.DialogCounter`))))
    (:`then`
      (bind (_name _expression _sfx _line) (break `/Game/BluePrint/ST_DialogSetup` _returnvalue))
      (set `self.Name` _name)
      (set `self.Expression` _expression)
      (set `self.SFX` _sfx)
      (set `self.Line` _line))))

(fn `GetScriptRow`
  (params (RowName :type Name))
  (bind _returnvalue (`|GetDataTableRow` (`self.DT_Script`) RowName)
    (:`then`
      (bind (_epecialevent _music _background) (break `/Game/BluePrint/ST_Script` _returnvalue))
      (set `self.Epecial Event` _epecialevent)
      (set `self.Music` _music)
      (set `self.Background` _background))))

(fn `NextDialogRow`
  (set `self.DialogCounter` (+ (`self.DialogCounter`) 1))
  (return))

(fn `NextScriptRow`
  (set `self.ScriptCounter` (+ (`self.ScriptCounter`) 1)))

(fn `Play Music`
  (bind _background_music (`self.Background Music`))
  (`/Engine/EditorBlueprintResources/StandardMacros.IsValid` (`self.Music`)
    (:`Is Valid`
      (`AudioComponent.SetSound` _background_music (`self.Music`))
      (`AudioComponent.FadeIn` _background_music 1.0 1.0 0.0 "Linear"))))

(fn `SetCharacterExpression`
  (bind _characterimage (`/Game/UI/WG_Character01.CharacterImage` (`/Game/UI/WG_Hud.WG_Character01` (`self.HudRef`))))
  (`Image.SetBrushFromTexture` _characterimage (`self.Expression`) false)
  (`Widget.SetVisibility` _characterimage "Visible"))

(fn `UserConstructionScript`)